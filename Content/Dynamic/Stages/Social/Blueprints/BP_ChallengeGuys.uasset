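; BP_ChallengeGuys is an AI pawn in the Social stage that repeatedly approaches the player to start a social challenge.
; On reaching the player, it activates the level's BP_SocialChallenge, or skips activation if one is already active.
; After activating, it polls until the player's InChallenge flag clears.
; In both cases it then moves to a random nearby reachable point, waits a few random seconds and loops back to approach again.
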(event Custom|Wander%20to%20Player
  (bind _socialchallenge (Variables|Default|GetSocialChallenge))
  (AI|AIMoveTo self "0, 0, 0" (Variables|Default|GetAs%20BP%20Social%20Character) 2e+01 true
    (:OnSuccess
      (if (Variables|/Game/Dynamic/Stages/Social/Blueprints/BP_SocialChallenge.BP_SocialChallenge_C|GetActive _socialchallenge)
        (Development|PrintString "active")
        (AI|AIMoveTo self (.RandomLocation (AI|Navigation|GetRandomReachablePointinRadius (Transformation|GetActorLocation) 8e+02 0 0)) 0 5.0 false
          (:OnSuccess
            _)
          (:OnFail
            _))
        (Utilities|FlowControl|Delay (Math|Random|RandomFloatinRange 3.0 6.0))
        (CallFunction|WandertoPlayer)
        (else
          (Default|Activate _socialchallenge)
          (if (Variables|/Game/Dynamic/Stages/Social/Blueprints/BP_SocialCharacter.BP_SocialCharacter_C|GetIn%20Challenge (Variables|Default|GetAs%20BP%20Social%20Character)) :!label _label
            (Utilities|FlowControl|Delay 0.2)
            (goto _label)
            (else
              (AI|AIMoveTo self (.RandomLocation (AI|Navigation|GetRandomReachablePointinRadius (Transformation|GetActorLocation) 8e+02 0 0)) 0 5.0 false
                (:OnSuccess
                  _)
                (:OnFail
                  _))
              (Utilities|FlowControl|Delay (Math|Random|RandomFloatinRange 3.0 6.0))
              (CallFunction|WandertoPlayer))))))))

(event EventBeginPlay
  (bind _asbp_social_character (Utilities|Casting|CastToBP_SocialCharacter (Game|GetPlayerCharacter 0)))
  (Variables|Default|SetAs%20BP%20Social%20Character _asbp_social_character)
  (CallFunction|WandertoPlayer)
  (bind _returnvalue (Actor|GetActorOfClass "/Game/Dynamic/Stages/Social/Blueprints/BP_SocialChallenge.BP_SocialChallenge_C"))
  (Variables|Default|SetSocialChallenge _returnvalue))

(fn ConstructionScript)