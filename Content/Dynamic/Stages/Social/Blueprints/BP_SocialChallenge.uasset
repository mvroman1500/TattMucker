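; Social-stage challenge target that drifts up and down and completes when a BP_EnergySphere stays overlapped long enough.
; A looping timeline moves it to random heights around its start, and BeginPlay also shows a WBP_Eat widget after a delay.
; While active, overlap runs a LengthOfTimer-scaled timeline that shrinks the mesh, pausing when overlap ends.
; Activate and completion toggle visibility and InChallenge on BP_SocialCharacter, with completion also calling CompleteChallenge.
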(event OnComponentBeginOverlap(Box)
  (params (OverlappedComponent :type Primitive%20Component%20Object%20Reference) (OtherActor :type Actor%20Object%20Reference) (OtherComp :type Primitive%20Component%20Object%20Reference) (OtherBodyIndex :type Integer) (bFromSweep :type Boolean) (SweepResult :type Hit%20Result%20Structure%20%28by%20ref%29))
  (bind _size_tl (Variables|Default|GetSize_TL))
  (if (and (Utilities|ClassIsChildOf (Utilities|GetClass OtherActor) "/Game/Dynamic/Stages/Social/Blueprints/BP_EnergySphere.BP_EnergySphere_C") (Variables|Default|GetActive))
    (Components|Timeline|SetPlayRate (Variables|Default|GetSize_TL) (/ 1.0 (Variables|Default|GetLength%20of%20Timer)))
    (bind _newtrack_0 (Timeline|Size_TL Play)
      (:Update
        (Transformation|SetRelativeScale3D (Variables|Default|GetStaticMesh) (Math|Vector|Lerp(Vector) "0.500000,0.250000,1.000000" "0.500000,0.250000,0.100000" _newtrack_0)))
      (:Finished
        (Development|PrintString "Complete!")
        (Components|Timeline|SetPlaybackPosition _size_tl 0.0 true true)
        (Variables|Default|SetActive false)
        (Audio|Components|Audio|Stop _size_tl)
        (Rendering|SetActorHiddenInGame true)
        (bind _returnvalue (Actor|GetActorOfClass "/Game/Dynamic/Stages/Social/Blueprints/BP_SocialCharacter.BP_SocialCharacter_C"))
        (Variables|/Game/Dynamic/Stages/Social/Blueprints/BP_SocialCharacter.BP_SocialCharacter_C|SetIn%20Challenge _returnvalue false)
        (Default|CompleteChallenge _returnvalue)))))

(event OnComponentEndOverlap(Box)
  (params (OverlappedComponent :type Primitive%20Component%20Object%20Reference) (OtherActor :type Actor%20Object%20Reference) (OtherComp :type Primitive%20Component%20Object%20Reference) (OtherBodyIndex :type Integer))
  (if (Utilities|ClassIsChildOf (Utilities|GetClass OtherActor) "/Game/Dynamic/Stages/Social/Blueprints/BP_EnergySphere.BP_EnergySphere_C")
    (Audio|Components|Audio|Stop (Variables|Default|GetSize_TL))))

(event Custom|BeginMovement
  (bind _returnvalue (Transformation|GetActorLocation))
  (Variables|Default|SetTarget%20Location (Math|Random|RandomFloatinRange (+ (Variables|Default|GetStart%20Height) -3e+02) (+ (Variables|Default|GetStart%20Height) 3e+02)) :!label _label)
  (Variables|Default|SetCurrent%20Location (.z (Transformation|GetActorLocation)))
  (bind _newtrack_0 (Timeline|UpandDown PlayFromStart)
    (:Update
      (Transformation|SetActorLocation (Math|Vector|MakeVector (.x _returnvalue) (.y _returnvalue) (Math|Float|Lerp (Variables|Default|GetCurrent%20Location) (Variables|Default|GetTarget%20Location) _newtrack_0)) false false))
    (:Finished
      (goto _label))))

(event Custom|Activate
  (Rendering|SetActorHiddenInGame false)
  (Variables|Default|SetActive true)
  (bind _returnvalue (Actor|GetActorOfClass "/Game/Dynamic/Stages/Social/Blueprints/BP_SocialCharacter.BP_SocialCharacter_C"))
  (Variables|/Game/Dynamic/Stages/Social/Blueprints/BP_SocialCharacter.BP_SocialCharacter_C|SetIn%20Challenge _returnvalue true))

(event EventBeginPlay
  (Variables|Default|SetStart%20Height (.z (Transformation|GetActorLocation)))
  (CallFunction|BeginMovement)
  (Utilities|FlowControl|Delay 2.0)
  (bind _returnvalue (UserInterface|CreateWidget "/Game/Dynamic/Stages/Health/WBP_Eat.WBP_Eat_C"))
  (UserInterface|Viewport|AddtoViewport _returnvalue 0))

(fn ConstructionScript)