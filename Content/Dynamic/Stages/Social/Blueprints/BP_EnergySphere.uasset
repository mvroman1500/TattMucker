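; BP_EnergySphere is a social-stage prop that bounces upward with a boing sound whenever BoostUp is called.
; On BeginPlay it reads the Cycle_Manager game instance's phase, becoming a laser pistol from phase two onward and a plain sphere before that.
; BoostUp applies a velocity-change impulse and raises the next sound's pitch, while a looping retriggerable delay steps it back down between boosts, within clamped limits.
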(event Custom|Boost%20Up
  (Physics|AddImpulse (Variables|Debug|GetStaticMeshComponent) "0.000000,0.000000,350.000000" "None" true)
  (Audio|PlaySound2D "/Game/Static/Audio/Social/Boing_Cue.Boing_Cue" 1.0 (Variables|Default|GetPitch) 0.0 0 0)
  (Utilities|FlowControl|Sequence
    (:then_0
      (Utilities|FlowControl|RetriggerableDelay 0.25 :!label _label)
      (Variables|Default|SetPitch (Math|Float|Clamp(Float) (+ (Variables|Default|GetPitch) -0.2) (Variables|Default|GetStarting%20Pitch) (Variables|Default|GetMax%20Pitch)))
      (goto _label))
    (:then_1
      (Variables|Default|SetPitch (Math|Float|Clamp(Float) (+ (Variables|Default|GetPitch) 0.1) (Variables|Default|GetStarting%20Pitch) (Variables|Default|GetMax%20Pitch))))))

(event EventBeginPlay
  (bind _ascycle_manager (Utilities|Casting|CastToCycle_Manager (Game|GetGameInstance)))
  (Components|StaticMesh|SetStaticMesh (Variables|Debug|GetStaticMeshComponent) (select (>= (Variables|/Game/Dynamic/Cycle_Manager.Cycle_Manager_C|GetPhase%20Number _ascycle_manager) 2) "/Game/Static/ImportedMeshes/LaserGun/SM_LaserPistol.SM_LaserPistol" "/Engine/BasicShapes/Sphere.Sphere"))
  (Rendering|Material|SetMaterial (Variables|Debug|GetStaticMeshComponent) 0 (select (>= (Variables|/Game/Dynamic/Cycle_Manager.Cycle_Manager_C|GetPhase%20Number _ascycle_manager) 2) "/Game/Static/ImportedMeshes/LaserGun/Material__25.Material__25" "/Game/StarterContent/Materials/M_Basic_Wall.M_Basic_Wall")))

(fn ConstructionScript)