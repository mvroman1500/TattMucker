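; Spawner for the Work stage that fills a rectangular area with BP_File actors at an accelerating rate and shows the WBP_Quota widget.
; After an initial batch, SpawnFiles re-calls itself after a delay, placing files randomly between the BottomLeft and TopRight markers.
; The Cycle_Manager phase number sets the spawn interval and how often a looping timer shortens it, within clamped limits.
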(event Custom|SpawnFiles
  (params (Number%20to%20Spawn :type Integer))
  (bind _topright (Variables|Default|GetTopRight))
  (bind _bottomleft (Variables|Default|GetBottomLeft))
  (bind _returnvalue (Transformation|GetWorldLocation _bottomleft))
  (bind _returnvalue_2 (Transformation|GetWorldLocation _topright))
  (for _index (range 0 Number%20to%20Spawn)
    (Game|SpawnActorfromClass "/Game/Dynamic/Stages/Work/Blueprints/BP_File.BP_File_C" (Math|Transform|MakeTransform (Math|Vector|MakeVector (Math|Random|RandomFloatinRange (.x _returnvalue) (.x _returnvalue_2)) (Math|Random|RandomFloatinRange (.y _returnvalue_2) (.y _returnvalue)) -1e+02)) "Undefined" "MultiplyWithRoot" 0 3 0))
  (Utilities|FlowControl|Delay (Variables|Default|GetTime%20Between%20Spawns))
  (CallFunction|SpawnFiles (Variables|Default|GetNumber%20of%20Spawns)))

(event EventBeginPlay
  (bind _asbp_work_character (Utilities|Casting|CastToBP_Work_Character (Game|GetPlayerCharacter 0)))
  (bind _returnvalue (UserInterface|CreateWidget "/Game/Dynamic/Stages/Work/UI/WBP_Quota.WBP_Quota_C" 0 (Variables|Default|GetQuota) _asbp_work_character))
  (UserInterface|Viewport|AddtoViewport _returnvalue 0)
  (CallFunction|SpawnFiles 5)
  (bind _ascycle_manager (Utilities|Casting|CastToCycle_Manager (Game|GetGameInstance)))
  (Variables|Default|SetTime%20Between%20Decrease%20of%20Time%20Between%20Spawns (Utilities|Select :Index (Variables|/Game/Dynamic/Cycle_Manager.Cycle_Manager_C|GetPhase%20Number _ascycle_manager) :Option%200 8.0 :Option%201 8.0 :Option%202 4.0 :Option%203 2.0))
  (Variables|Default|SetTime%20Between%20Spawns (Utilities|Select :Index (Variables|/Game/Dynamic/Cycle_Manager.Cycle_Manager_C|GetPhase%20Number _ascycle_manager) :Option%200 5.0 :Option%201 5.0 :Option%202 3.0 :Option%203 2.0))
  (Utilities|Time|SetTimerbyFunctionName 0 "Decrease Time" (Variables|Default|GetTime%20Between%20Decrease%20of%20Time%20Between%20Spawns) true))

(fn ConstructionScript)

(fn DecreaseTime
  (Variables|Default|SetTime%20Between%20Spawns (Math|Float|Clamp(Float) (- (Variables|Default|GetTime%20Between%20Spawns) (Variables|Default|GetDecrease%20Amount)) 0.3 5.0)))