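; BP_Bin is a clickable trash bin in the work stage where the player disposes of a held file.
; On click it lazily caches the work character and, if an object is held, clears the holding flag, destroys the file and increments the character's Completed count.
; It then plays a paper-trash sound while a sped-up timeline drives the cylinder's yaw for a shake.
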(event Custom|Animation
  (Components|Timeline|SetPlayRate (Variables|Default|GetTimeline) 2.0)
  (Audio|PlaySound2D "/Game/Static/Audio/Work/PaperThrownIntoTrash_Cue.PaperThrownIntoTrash_Cue" 0.7 1.0 0.0 0 0)
  (bind _shake (Timeline|Timeline PlayFromStart)
    (:Update
      (Transformation|SetRelativeRotation (Variables|Default|GetCylinder) (Math|Rotator|MakeRotator 0.0 0.0 (Math|Float|Lerp 0.0 3e+01 _shake)) false false))))

(event MouseInput|EventActorOnClicked
  (params (ButtonPressed :type Key%20Structure :default "None"))
  (Utilities|IsValid (Variables|Default|GetAs%20BP%20Work%20Character)
    (:Is%20Valid
      _)
    (:Is%20Not%20Valid
      (bind _asbp_work_character (Utilities|Casting|CastToBP_Work_Character (Game|GetPlayerCharacter 0)))
      (Variables|Default|SetAs%20BP%20Work%20Character _asbp_work_character)))
  (if (Variables|/Game/Dynamic/Stages/Work/BP_Work_Character.BP_Work_Character_C|GetHolding%20An%20Object (Variables|Default|GetAs%20BP%20Work%20Character))
    (Variables|/Game/Dynamic/Stages/Work/BP_Work_Character.BP_Work_Character_C|SetHolding%20An%20Object (Variables|Default|GetAs%20BP%20Work%20Character) false)
    (Actor|DestroyActor (Variables|/Game/Dynamic/Stages/Work/BP_Work_Character.BP_Work_Character_C|GetHeld%20FIle (Variables|Default|GetAs%20BP%20Work%20Character)))
    (bind _result (Math|Integer|IncrementInt (Variables|/Game/Dynamic/Stages/Work/BP_Work_Character.BP_Work_Character_C|GetCompleted (Variables|Default|GetAs%20BP%20Work%20Character)))
      (:%20%20
        (Variables|/Game/Dynamic/Stages/Work/BP_Work_Character.BP_Work_Character_C|SetCompleted (Variables|Default|GetAs%20BP%20Work%20Character) _result)
        (CallFunction|Animation)))))

(fn ConstructionScript)