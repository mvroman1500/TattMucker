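; Clickable file actor for the work stage, labelled with a random message from a pool that widens in later Cycle_Manager phases.
; From phase four it can randomly become an alien file that explodes with sounds when clicked empty-handed.
; Otherwise, clicking registers it as BP_Work_Character's held file, disables its collision and makes it follow the deprojected mouse position at fixed height on Tick.
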(event EventTick
  (params (DeltaSeconds :type Float%20%28single-precision%29))
  (bind _returnvalue (Game|GetPlayerController 0))
  (bind _worldlocation (Game|Player|ConvertMouseLocationToWorldSpace _returnvalue))
  (if (Variables|Default|GetPicked%20Up)
    (Transformation|SetActorLocation (Math|Vector|MakeVector (.x _worldlocation) (.y _worldlocation) -1e+02) false false)))

(event MouseInput|EventActorOnClicked
  (params (ButtonPressed :type Key%20Structure :default "None"))
  (Development|PrintString "Hello")
  (bind _asbp_work_character (Utilities|Casting|CastToBP_Work_Character (Game|GetPlayerCharacter 0)))
  (if (not (Variables|/Game/Dynamic/Stages/Work/BP_Work_Character.BP_Work_Character_C|GetHolding%20An%20Object _asbp_work_character))
    (if (Variables|Default|GetAlien%20Mode)
      (Effects|SpawnEmitteratLocation "/Game/StarterContent/Particles/P_Explosion.P_Explosion" (Transformation|GetActorLocation))
      (Audio|PlaySound2D "/Game/Static/Audio/Fun/SC_AlienDeath.SC_AlienDeath" 1.0 1.0 0.0 0 0)
      (Audio|PlaySound2D "/Game/StarterContent/Audio/Explosion_Cue.Explosion_Cue" 0.2 1.0 0.0 0 0)
      (Actor|DestroyActor)
      (else
        (Variables|/Game/Dynamic/Stages/Work/BP_Work_Character.BP_Work_Character_C|SetHolding%20An%20Object _asbp_work_character true)
        (Variables|/Game/Dynamic/Stages/Work/BP_Work_Character.BP_Work_Character_C|SetHeld%20FIle _asbp_work_character self)
        (Variables|Default|SetPicked%20Up true)
        (Collision|SetActorEnableCollision false)))))

(event EventBeginPlay
  (bind _ascycle_manager (Utilities|Casting|CastToCycle_Manager (Game|GetGameInstance)))
  (Variables|Default|SetAs%20Cycle%20Manager _ascycle_manager)
  (if (>= (Variables|/Game/Dynamic/Cycle_Manager.Cycle_Manager_C|GetPhase%20Number _ascycle_manager) 4)
    (if (> (Math|Random|RandomIntegerinRange 0 7) 5)
      (Rendering|Components|TextRender|SetText (Variables|Default|GetTextRender) (Utilities|Text|MakeLiteralText "BLEHHH"))
      (Rendering|Material|SetMaterial (Variables|Default|GetCube) 0 "/Game/Static/Textures/M_Alien.M_Alien")
      (Variables|Default|SetAlien%20Mode true)
      (else
        (Variables|Default|SetTextOptions (Utilities|Select :Index (- (Variables|/Game/Dynamic/Cycle_Manager.Cycle_Manager_C|GetPhase%20Number _ascycle_manager) 1) :Option%200 3 :Option%201 3 :Option%202 3 :Option%203 5 :Option%204 5 :Option%205 5) :!label _label)))
    (else
      (goto _label)))
  (Rendering|Components|TextRender|SetText (Variables|Default|GetTextRender) (Utilities|Select :Index (Math|Random|RandomIntegerinRange 0 (Variables|Default|GetTextOptions)) :Option%200 (Utilities|Text|MakeLiteralText "IMPORTANT") :Option%201 (Utilities|Text|MakeLiteralText "VERY IMPORTANT") :Option%202 (Utilities|Text|MakeLiteralText "AHHHHH") :Option%203 (Utilities|Text|MakeLiteralText "MANDATORY OVERTIME") :Option%204 (Utilities|Text|MakeLiteralText "your friends miss you.") :Option%205 (Utilities|Text|MakeLiteralText "you haven't eaten today.")))
  (Rendering|SetActorHiddenInGame false))

(fn ConstructionScript)