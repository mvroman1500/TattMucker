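; BP_RailSpawner spawns targets in the Fun stage, in staggered waves of three that arrive progressively faster.
; A timeline acts as the wave timer, its play rate rescaled as TimeToSpawn shrinks toward a floor.
; SpawnTarget draws spawn points randomly without replacement, refilling the pool when empty.
; Cycle_Manager phase 3 onward starts faster and spawns only file targets; earlier phases roll weighted small, medium or large targets, with one roll spawning nothing.
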(event Custom|SetPlayRate
  (bind _spawnertimeline (Variables|Default|GetSpawnerTimeline))
  (Components|Timeline|SetPlayRate (Variables|Default|GetSpawnerTimeline) 1.0)
  (Components|Timeline|SetPlayRate _spawnertimeline (/ (Components|Animation|GetPlayRate _spawnertimeline) (Variables|Default|GetTimeToSpawn))))

(event EventBeginPlay
  (Variables|Default|SetTimeToSpawn 5.0)
  (bind _ascycle_manager (Utilities|Casting|CastToCycle_Manager (Game|GetGameInstance)))
  (Variables|Default|SetAs%20Cycle%20Manager _ascycle_manager)
  (bind _asbp_fun_character (Utilities|Casting|CastToBP_FunCharacter (Game|GetPlayerCharacter 0)))
  (Variables|Default|SetAs%20BP%20Fun%20Character _asbp_fun_character)
  (Variables|Default|SetFirstSpawn? true)
  (Variables|Default|SetAllSpawnLocations (Utilities|Array|MakeArray (Variables|SpawnPoints|GetSpawnPoint7) (Variables|SpawnPoints|GetSpawnPoint13) (Variables|SpawnPoints|GetSpawnPoint8) (Variables|SpawnPoints|GetSpawnPoint9) (Variables|SpawnPoints|GetSpawnPoint6) (Variables|SpawnPoints|GetSpawnPoint10) (Variables|SpawnPoints|GetSpawnPoint11) (Variables|SpawnPoints|GetSpawnPoint12) (Variables|SpawnPoints|GetSpawnPoint5) (Variables|SpawnPoints|GetSpawnPoint) (Variables|SpawnPoints|GetSpawnPoint4) (Variables|SpawnPoints|GetSpawnPoint3) (Variables|SpawnPoints|GetSpawnPoint2) (Variables|SpawnPoints|GetSpawnPoint1)))
  (Variables|Default|SetCurrentAvailableSpawnLocations (Utilities|Array|MakeArray (Variables|SpawnPoints|GetSpawnPoint7) (Variables|SpawnPoints|GetSpawnPoint13) (Variables|SpawnPoints|GetSpawnPoint8) (Variables|SpawnPoints|GetSpawnPoint9) (Variables|SpawnPoints|GetSpawnPoint6) (Variables|SpawnPoints|GetSpawnPoint10) (Variables|SpawnPoints|GetSpawnPoint11) (Variables|SpawnPoints|GetSpawnPoint12) (Variables|SpawnPoints|GetSpawnPoint5) (Variables|SpawnPoints|GetSpawnPoint) (Variables|SpawnPoints|GetSpawnPoint4) (Variables|SpawnPoints|GetSpawnPoint3) (Variables|SpawnPoints|GetSpawnPoint2) (Variables|SpawnPoints|GetSpawnPoint1)))
  (if (Variables|Default|GetFirstSpawn?)
    (if (>= (Variables|/Game/Dynamic/Cycle_Manager.Cycle_Manager_C|GetPhase%20Number (Variables|Default|GetAs%20Cycle%20Manager)) 3)
      (Variables|Default|SetTimeToSpawn 3.0))
    (CallFunction|SpawnTarget)
    (Utilities|FlowControl|Delay 0.2)
    (CallFunction|SpawnTarget)
    (Utilities|FlowControl|Delay 0.2)
    (CallFunction|SpawnTarget)
    (Variables|Default|SetFirstSpawn? false)
    (CallFunction|SetPlayRate)
    (Timeline|SpawnerTimeline PlayFromStart
      (:Finished
        (if (>= (Variables|Default|GetTimeToSpawn) 0.26)
          (bind _output_get (Variables|Default|SetTimeToSpawn (- (Variables|Default|GetTimeToSpawn) 0.25)))
          (Development|PrintString (Utilities|String|ToString(Float) _output_get) true true "(R=0.000000,G=1.000000,B=0.189927,A=1.000000)")
          (Utilities|FlowControl|Sequence
            (:then_0
              (CallFunction|SetPlayRate))
            (:then_1
              (CallFunction|SpawnTarget :!label _label)
              (Utilities|FlowControl|Delay 0.2)
              (CallFunction|SpawnTarget)
              (Utilities|FlowControl|Delay 0.2)
              (CallFunction|SpawnTarget)
              (Timeline|SpawnerTimeline PlayFromStart)))
          (else
            (goto _label)))))))

(fn ConstructionScript)

(fn SpawnTarget
  (bind _currentavailablespawnlocations (Variables|Default|GetCurrentAvailableSpawnLocations))
  (bind _currentavailablespawnlocations_2 (Variables|Default|GetCurrentAvailableSpawnLocations))
  (bind (_outitem _outindex) (Utilities|Array|Random _currentavailablespawnlocations_2))
  (if (== _outindex -1)
    (CallFunction|RefillTargets)
    (bind _output_get (Variables|Default|SetSelectedSpawnLoaction (.OutItem (Utilities|Array|Random _currentavailablespawnlocations))))
    (Utilities|Array|RemoveItem _currentavailablespawnlocations _output_get)
    (else
      (bind _output_get_2 (Variables|Default|SetSelectedSpawnLoaction _outitem))
      (Utilities|Array|RemoveItem _currentavailablespawnlocations_2 _output_get_2)))
  (if (>= (Variables|/Game/Dynamic/Cycle_Manager.Cycle_Manager_C|GetPhase%20Number (Variables|Default|GetAs%20Cycle%20Manager)) 3)
    (Game|SpawnActorfromClass "/Game/Dynamic/Stages/Fun/Blueprints/BP_FileTarget.BP_FileTarget_C" (Math|Transform|MakeTransform (Math|Vector|MakeVector (.x (Transformation|GetWorldLocation _output_get_2)) (.y (Transformation|GetWorldLocation _output_get_2)) (+ (.z (Transformation|GetWorldLocation _output_get_2)) (Variables|Default|GetZOffset))) (Transformation|GetWorldRotation _output_get_2) "1.000000,1.000000,1.000000") "Undefined" "MultiplyWithRoot" 0 0)
    (else
      (switch int (Math|Random|RandomIntegerinRange 0 9)
        (:0
          (Game|SpawnActorfromClass "/Game/Dynamic/Stages/Fun/Blueprints/BP_TargetSmall.BP_TargetSmall_C" (Math|Transform|MakeTransform (Math|Vector|MakeVector (.x (Transformation|GetWorldLocation _output_get_2)) (.y (Transformation|GetWorldLocation _output_get_2)) (+ (.z (Transformation|GetWorldLocation _output_get_2)) (Variables|Default|GetZOffset))) (Transformation|GetWorldRotation _output_get_2) "1.000000,1.000000,1.000000") "Undefined" "MultiplyWithRoot" 0 0 :!label _label))
        (:1
          (goto _label))
        (:2
          (goto _label))
        (:3
          (goto _label))
        (:4
          (Game|SpawnActorfromClass "/Game/Dynamic/Stages/Fun/Blueprints/BP_TargetMed.BP_TargetMed_C" (Math|Transform|MakeTransform (Math|Vector|MakeVector (.x (Transformation|GetWorldLocation _output_get_2)) (.y (Transformation|GetWorldLocation _output_get_2)) (+ (.z (Transformation|GetWorldLocation _output_get_2)) (Variables|Default|GetZOffset))) (Transformation|GetWorldRotation _output_get_2) "1.000000,1.000000,1.000000") "Undefined" "MultiplyWithRoot" 0 0 :!label _label_2))
        (:5
          (goto _label_2))
        (:6
          (goto _label_2))
        (:7
          (Game|SpawnActorfromClass "/Game/Dynamic/Stages/Fun/Blueprints/BP_TargetLarge.BP_TargetLarge_C" (Math|Transform|MakeTransform (Math|Vector|MakeVector (.x (Transformation|GetWorldLocation _output_get_2)) (.y (Transformation|GetWorldLocation _output_get_2)) (+ (.z (Transformation|GetWorldLocation _output_get_2)) (Variables|Default|GetZOffset))) (Transformation|GetWorldRotation _output_get_2) "1.000000,1.000000,1.000000") "Undefined" "MultiplyWithRoot" 0 0 :!label _label_3))
        (:8
          (goto _label_3))))))

(fn RefillTargets
  (Variables|Default|SetCurrentAvailableSpawnLocations (Utilities|Array|MakeArray (Variables|SpawnPoints|GetSpawnPoint7) (Variables|SpawnPoints|GetSpawnPoint13) (Variables|SpawnPoints|GetSpawnPoint8) (Variables|SpawnPoints|GetSpawnPoint9) (Variables|SpawnPoints|GetSpawnPoint6) (Variables|SpawnPoints|GetSpawnPoint10) (Variables|SpawnPoints|GetSpawnPoint11) (Variables|SpawnPoints|GetSpawnPoint12) (Variables|SpawnPoints|GetSpawnPoint5) (Variables|SpawnPoints|GetSpawnPoint) (Variables|SpawnPoints|GetSpawnPoint4) (Variables|SpawnPoints|GetSpawnPoint3) (Variables|SpawnPoints|GetSpawnPoint2) (Variables|SpawnPoints|GetSpawnPoint1))))