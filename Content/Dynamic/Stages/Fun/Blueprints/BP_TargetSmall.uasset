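; BP_TargetSmall is a small target actor in the Fun stage that is knocked out when something overlaps its trigger box.
; The first box overlap passes a DoOnce gate and calls KillSmall.
; KillSmall plays the Kill timeline, which lerps the Scene component 150 units downward, then destroys the actor when it finishes.
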(event OnComponentBeginOverlap(Box)
  (params (OverlappedComponent :type Primitive%20Component%20Object%20Reference) (OtherActor :type Actor%20Object%20Reference) (OtherComp :type Primitive%20Component%20Object%20Reference) (OtherBodyIndex :type Integer) (bFromSweep :type Boolean) (SweepResult :type Hit%20Result%20Structure%20%28by%20ref%29))
  (Utilities|FlowControl|DoOnce false
    (:Completed
      (CallFunction|KillSmall))))

(event Custom|KillSmall
  (bind _scene (Variables|Default|GetScene))
  (bind _returnvalue (Transformation|GetWorldLocation _scene))
  (bind _newtrack_0 (Timeline|Kill Play)
    (:Update
      (Transformation|SetWorldLocation _scene (Math|Vector|MakeVector (.x _returnvalue) (.y _returnvalue) (Math|Float|Lerp (.z _returnvalue) (- (.z _returnvalue) 1.5e+02) _newtrack_0)) false false))
    (:Finished
      (Actor|DestroyActor))))

(event EventBeginPlay
  (|CallParentFunction) ; This node is disabled and will not be called.\nDrag off pins to build functionality.
)

(event Collision|EventActorBeginOverlap
  (params (OtherActor :type Actor%20Object%20Reference))
  (|CallParentFunction OtherActor) ; This node is disabled and will not be called.\nDrag off pins to build functionality.
)

(event EventTick
  (params (DeltaSeconds :type Float%20%28single-precision%29))
  (|CallParentFunction DeltaSeconds) ; This node is disabled and will not be called.\nDrag off pins to build functionality.
)

(fn ConstructionScript
  (|CallParentFunction))