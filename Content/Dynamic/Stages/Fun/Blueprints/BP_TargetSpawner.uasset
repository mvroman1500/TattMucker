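; BP_TargetSpawner is an actor that populates an area of the Fun stage with three targets at BeginPlay.
; Each spawn picks a random class from Targets and a random location bounded by marker components: Back/Front for X, Left/Right for both Y and Z.
; After each spawn it increments TargetsRemaining on the player's BP_FunCharacter; nothing spawns if that cast fails.
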(event Custom|SpawnInRandomArea
  (bind _left (Variables|Default|GetLeft))
  (bind _right (Variables|Default|GetRight))
  (bind _returnvalue (Transformation|GetWorldLocation _right))
  (bind _returnvalue_2 (Transformation|GetWorldLocation _left))
  (Game|SpawnActorfromClass (.OutItem (Utilities|Array|Random (Variables|Default|GetTargets))) (Math|Transform|MakeTransform (Math|Vector|MakeVector (Math|Random|RandomFloatinRange (.x (Transformation|GetWorldLocation (Variables|Default|GetBack))) (.x (Transformation|GetWorldLocation (Variables|Default|GetFront)))) (Math|Random|RandomFloatinRange (.y _returnvalue_2) (.y _returnvalue)) (Math|Random|RandomFloatinRange (.z _returnvalue_2) (.z _returnvalue)))) "Undefined" "MultiplyWithRoot" 0 0))

(event EventBeginPlay
  (bind _asbp_fun_character (Utilities|Casting|CastToBP_FunCharacter (Game|GetPlayerCharacter 0)))
  (Variables|Default|SetAs%20BP%20Fun%20Character _asbp_fun_character)
  (CallFunction|SpawninRandomArea)
  (bind _result (Math|Integer|IncrementInt (Variables|/Game/Dynamic/Stages/Fun/Blueprints/BP_FunCharacter.BP_FunCharacter_C|GetTargetsRemaining (Variables|Default|GetAs%20BP%20Fun%20Character)))
    (:%20%20
      (Variables|/Game/Dynamic/Stages/Fun/Blueprints/BP_FunCharacter.BP_FunCharacter_C|SetTargetsRemaining (Variables|Default|GetAs%20BP%20Fun%20Character) _result)
      (CallFunction|SpawninRandomArea)
      (bind _result_2 (Math|Integer|IncrementInt (Variables|/Game/Dynamic/Stages/Fun/Blueprints/BP_FunCharacter.BP_FunCharacter_C|GetTargetsRemaining (Variables|Default|GetAs%20BP%20Fun%20Character)))
        (:%20%20
          (Variables|/Game/Dynamic/Stages/Fun/Blueprints/BP_FunCharacter.BP_FunCharacter_C|SetTargetsRemaining (Variables|Default|GetAs%20BP%20Fun%20Character) _result_2)
          (CallFunction|SpawninRandomArea)
          (bind _result_3 (Math|Integer|IncrementInt (Variables|/Game/Dynamic/Stages/Fun/Blueprints/BP_FunCharacter.BP_FunCharacter_C|GetTargetsRemaining (Variables|Default|GetAs%20BP%20Fun%20Character)))
            (:%20%20
              (Variables|/Game/Dynamic/Stages/Fun/Blueprints/BP_FunCharacter.BP_FunCharacter_C|SetTargetsRemaining (Variables|Default|GetAs%20BP%20Fun%20Character) _result_3))))))))

(fn ConstructionScript)