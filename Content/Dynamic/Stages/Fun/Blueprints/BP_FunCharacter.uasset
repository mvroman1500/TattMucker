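; Player character for the Fun stage, a first-person shooter with look and shoot input and a clamped camera view.
; Shooting spawns BP_GunProjectile from the pistol's Ammo socket along camera rotation, gated by a short cooldown, with chained timelines for recoil.
; BeginPlay adds the input mapping and creates the HUD, which UpdateScore refreshes.
; Hard-coded branches always use the WorkFunCrossover quota widget; phase checks and fire sound are disconnected.
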(event Custom|UpdateScore
  (if true
    (Default|SetQuotaText (Variables|Default|GetQuotaRef))
    (else
      (Default|SetScoreText (Variables|Default|GetScoreRef)))))

(event Custom|Reverse%20Movment
  (bind _sm_laserpistol1 (Variables|Default|GetSM_LaserPistol1))
  (bind _relativelocation (Variables|/Script/Engine.SceneComponent|GetRelativeLocation _sm_laserpistol1))
  (bind _gunmovement (Timeline|Timeline PlayFromStart)
    (:Update
      (Transformation|SetRelativeLocation _sm_laserpistol1 (Math|Vector|MakeVector (+ (.x _gunmovement) (.x _relativelocation)) (.y _relativelocation) (.z _relativelocation)) false false))))

(event Custom|StartMovement
  (bind _sm_laserpistol1 (Variables|Default|GetSM_LaserPistol1))
  (bind _relativelocation (Variables|/Script/Engine.SceneComponent|GetRelativeLocation _sm_laserpistol1))
  (bind _gunmovement (Timeline|MoveGun PlayFromStart)
    (:Update
      (Transformation|SetRelativeLocation _sm_laserpistol1 (Math|Vector|MakeVector (- (.x _relativelocation) (.x _gunmovement)) (.y _relativelocation) (.z _relativelocation)) false false))
    (:Finished
      (CallFunction|ReverseMovment))))

(event Input|EnhancedActionEvents|EnhancedInputActionIA_Look
  (params (ActionValue :type Vector%202D%20Structure) (ElapsedSeconds :type Float%20%28double-precision%29) (TriggeredSeconds :type Float%20%28double-precision%29) (InputAction :type Input%20Action%20Object%20Reference :default "/Game/Dynamic/Stages/Fun/Inputs/IA_Look.IA_Look"))
  (Pawn|Input|AddControllerYawInput (.x ActionValue))
  (Pawn|Input|AddControllerPitchInput (.y ActionValue)))

(event Input|EnhancedActionEvents|EnhancedInputActionIA_Shoot
  (params (ActionValue :type Boolean) (ElapsedSeconds :type Float%20%28double-precision%29) (TriggeredSeconds :type Float%20%28double-precision%29) (InputAction :type Input%20Action%20Object%20Reference :default "/Game/Dynamic/Stages/Fun/Inputs/IA_Shoot.IA_Shoot"))
  (bind _returnvalue (Game|GetPlayerCameraManager 0))
  (bind _projectileoffset (Variables|Projectile|GetProjectileOffset))
  (bind _sm_laserpistol1 (Variables|Default|GetSM_LaserPistol1))
  (bind _returnvalue_2 (Transformation|GetSocketLocation _sm_laserpistol1 "Ammo"))
  (bind _returnvalue_3 (Camera|GetCameraRotation _returnvalue))
  (bind _returnvalue_4 (Math|Vector|RotateVector _projectileoffset _returnvalue_3))
  (bind _returnvalue_5 (+ _returnvalue_2 _returnvalue_4))
  (bind _returnvalue_6 (Math|Transform|MakeTransform _returnvalue_5 _returnvalue_3))
  (:Started
    (if (Variables|Default|GetcanFire)
      (bind _returnvalue_7 (Game|SpawnActorfromClass "/Game/Dynamic/Stages/Fun/Blueprints/BP_GunProjectile.BP_GunProjectile_C" (Math|Transform|MakeTransform (.location _returnvalue_6) (Math|Rotator|MakeRotator (.roll (.rotation _returnvalue_6)) (.pitch (.rotation _returnvalue_6)) (.yaw (.rotation _returnvalue_6))) (.scale _returnvalue_6)) "Undefined" "MultiplyWithRoot" 0 0))
      (CallFunction|StartMovement)
      (Variables|Default|SetcanFire false)
      (Utilities|FlowControl|Delay 0.15)
      (Variables|Default|SetcanFire true))))

(event EventBeginPlay
  (bind _returnvalue (Game|GetPlayerCameraManager 0))
  (Input|SetInputModeGameOnly (Game|GetPlayerController 0) false)
  (bind _asplayer_controller (Utilities|Casting|CastToPlayerController (Pawn|GetController)))
  (Utilities|IsValid (PlayerController|LocalPlayerSubsystems|GetEnhancedInputLocalPlayerSubsystem _asplayer_controller)
    (:Is%20Valid
      (Input|AddMappingContext (PlayerController|LocalPlayerSubsystems|GetEnhancedInputLocalPlayerSubsystem _asplayer_controller) "/Game/Dynamic/Stages/Fun/Inputs/IMC_Fun.IMC_Fun" 0 "(bIgnoreAllPressedKeysUntilRelease=True,bForceImmediately=False,bNotifyUserSettings=False)")
      (Variables|/Script/Engine.PlayerCameraManager|SetViewPitchMax _returnvalue 35.0)
      (Variables|/Script/Engine.PlayerCameraManager|SetViewPitchMin _returnvalue -5.0)
      (Variables|/Script/Engine.PlayerCameraManager|SetViewYawMax _returnvalue 35.0)
      (Variables|/Script/Engine.PlayerCameraManager|SetViewYawMin _returnvalue -35.0)
      (bind _ascycle_manager (Utilities|Casting|CastToCycle_Manager (Game|GetGameInstance)))
      (bind _output_get (Variables|Default|SetCycleManagerRef _ascycle_manager))
      (if true
        (bind _returnvalue_2 (UserInterface|CreateWidget "/Game/Dynamic/Stages/Fun/UI/WBP_WorkFunCrossover.WBP_WorkFunCrossover_C"))
        (bind _output_get_2 (Variables|Default|SetQuotaRef _returnvalue_2))
        (UserInterface|Viewport|AddtoViewport _output_get_2 0)
        (else
          (bind _returnvalue_3 (UserInterface|CreateWidget "/Game/Dynamic/Stages/Fun/UI/WBP_FunScore.WBP_FunScore_C"))
          (bind _output_get_3 (Variables|Default|SetScoreRef _returnvalue_3))
          (UserInterface|Viewport|AddtoViewport _output_get_3 0))))))

(fn ConstructionScript)