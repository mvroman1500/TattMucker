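; BP_TargetLarge is a large target that may slide side to side along Y and drops away when hit.
; After a short delay at BeginPlay, a random roll either starts movement using BP_MoveBounds limits or leaves it still.
; The Movement timeline alternates forward and reverse via a FlipFlop, with JustSpawned making the first pass begin at the spawn position.
; The first Box overlap stops movement and plays the Kill timeline, which lowers the target.
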(event OnComponentBeginOverlap(Box)
  (params (OverlappedComponent :type Primitive%20Component%20Object%20Reference) (OtherActor :type Actor%20Object%20Reference) (OtherComp :type Primitive%20Component%20Object%20Reference) (OtherBodyIndex :type Integer) (bFromSweep :type Boolean) (SweepResult :type Hit%20Result%20Structure%20%28by%20ref%29))
  (Utilities|FlowControl|DoOnce false
    (:Completed
      (CallFunction|KillLarge))))

(event Custom|StartMoving
  (bind _scene (Variables|Default|GetScene))
  (bind _levelboundsref (Variables|Default|GetLevelBoundsRef))
  (bind _scene_2 (Variables|Default|GetScene))
  (bind _returnvalue (Transformation|GetWorldLocation _scene_2))
  (bind _returnvalue_2 (Transformation|GetWorldLocation _scene))
  (bind _moveyaxis (Timeline|Movement Play)
    (:Update
      (if (Variables|Default|GetJustSpawned)
        (Transformation|SetWorldLocation _scene (Math|Vector|MakeVector (.x _returnvalue_2) (Math|Float|Lerp (Variables|Default|GetStartYLocation) (Variables|/Game/Dynamic/Stages/Fun/Blueprints/BP_MoveBounds.BP_MoveBounds_C|GetRightBoundsY (Variables|Default|GetLevelBoundsRef)) _moveyaxis) (.z _returnvalue_2)) false false)
        (else
          (Transformation|SetWorldLocation _scene_2 (Math|Vector|MakeVector (.x _returnvalue) (Math|Float|Lerp (Variables|/Game/Dynamic/Stages/Fun/Blueprints/BP_MoveBounds.BP_MoveBounds_C|GetLeftBoundsY _levelboundsref) (Variables|/Game/Dynamic/Stages/Fun/Blueprints/BP_MoveBounds.BP_MoveBounds_C|GetRightBoundsY _levelboundsref) _moveyaxis) (.z _returnvalue)) false false))))
    (:Finished
      (Utilities|FlowControl|FlipFlop
        (:A
          (Variables|Default|SetJustSpawned false)
          (CallFunction|ReverseMovement))
        (:B
          (CallFunction|StartMoving))))))

(event Custom|ReverseMovement
  (bind _scene (Variables|Default|GetScene))
  (bind _levelboundsref (Variables|Default|GetLevelBoundsRef))
  (bind _scene_2 (Variables|Default|GetScene))
  (bind _returnvalue (Transformation|GetWorldLocation _scene_2))
  (bind _returnvalue_2 (Transformation|GetWorldLocation _scene))
  (bind _moveyaxis (Timeline|Movement ReverseFromEnd)
    (:Update
      (if (Variables|Default|GetJustSpawned)
        (Transformation|SetWorldLocation _scene (Math|Vector|MakeVector (.x _returnvalue_2) (Math|Float|Lerp (Variables|Default|GetStartYLocation) (Variables|/Game/Dynamic/Stages/Fun/Blueprints/BP_MoveBounds.BP_MoveBounds_C|GetRightBoundsY (Variables|Default|GetLevelBoundsRef)) _moveyaxis) (.z _returnvalue_2)) false false)
        (else
          (Transformation|SetWorldLocation _scene_2 (Math|Vector|MakeVector (.x _returnvalue) (Math|Float|Lerp (Variables|/Game/Dynamic/Stages/Fun/Blueprints/BP_MoveBounds.BP_MoveBounds_C|GetLeftBoundsY _levelboundsref) (Variables|/Game/Dynamic/Stages/Fun/Blueprints/BP_MoveBounds.BP_MoveBounds_C|GetRightBoundsY _levelboundsref) _moveyaxis) (.z _returnvalue)) false false))))
    (:Finished
      (Utilities|FlowControl|FlipFlop
        (:A
          (Variables|Default|SetJustSpawned false)
          (CallFunction|ReverseMovement))
        (:B
          (CallFunction|StartMoving))))))

(event Custom|KillLarge
  (bind _scene (Variables|Default|GetScene))
  (bind _returnvalue (Transformation|GetWorldLocation _scene))
  (Audio|Components|Audio|Stop (Variables|Default|GetMovement))
  (bind _newtrack_0 (Timeline|Kill Play)
    (:Update
      (Transformation|SetWorldLocation _scene (Math|Vector|MakeVector (.x _returnvalue) (.y _returnvalue) (Math|Float|Lerp (.z _returnvalue) (- (.z _returnvalue) 1.5e+02) _newtrack_0)) false false))))

(event EventBeginPlay
  (|CallParentFunction)
  (Utilities|FlowControl|Delay 1.0)
  (Variables|Default|SetStartYLocation (.y (Transformation|GetWorldLocation (Variables|Default|GetScene))))
  (switch int (Math|Random|RandomIntegerinRange 0 2)
    (:0
      (bind _returnvalue (Actor|GetActorOfClass "/Game/Dynamic/Stages/Fun/Blueprints/BP_MoveBounds.BP_MoveBounds_C"))
      (Variables|Default|SetLevelBoundsRef _returnvalue)
      (CallFunction|StartMoving))
    (:1
      (bind _returnvalue_2 (Actor|GetActorOfClass "/Game/Dynamic/Stages/Fun/Blueprints/BP_MoveBounds.BP_MoveBounds_C"))
      (Variables|Default|SetLevelBoundsRef _returnvalue_2)
      (CallFunction|StartMoving))))

(event Collision|EventActorBeginOverlap
  (params (OtherActor :type Actor%20Object%20Reference))
  (|CallParentFunction OtherActor) ; This node is disabled and will not be called.\nDrag off pins to build functionality.
)

(event EventTick
  (params (DeltaSeconds :type Float%20%28single-precision%29))
  (|CallParentFunction DeltaSeconds) ; This node is disabled and will not be called.\nDrag off pins to build functionality.
)

(fn ConstructionScript
  (|CallParentFunction))