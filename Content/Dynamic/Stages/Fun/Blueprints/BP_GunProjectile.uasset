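; BP_GunProjectile is the gun projectile for the Fun stage, scoring hits on tagged targets.
; On BeginPlay it caches the player's BP_FunCharacter.
; When its sphere overlaps a Small, Med or Large tagged actor, it destroys that target, plays a collapse sound, adds size-based score through the character and decrements its remaining target count.
; The projectile destroys itself on any overlap, printing a debug message for the result.
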(event OnComponentBeginOverlap(Sphere)
  (params (OverlappedComponent :type Primitive%20Component%20Object%20Reference) (OtherActor :type Actor%20Object%20Reference) (OtherComp :type Primitive%20Component%20Object%20Reference) (OtherBodyIndex :type Integer) (bFromSweep :type Boolean) (SweepResult :type Hit%20Result%20Structure%20%28by%20ref%29))
  (bind _as_bp_fun_character (Variables|Default|GetAs%20BP%20Fun%20Character))
  (bind _as_bp_fun_character_2 (Variables|Default|GetAs%20BP%20Fun%20Character))
  (bind _as_bp_fun_character_3 (Variables|Default|GetAs%20BP%20Fun%20Character))
  (if (Actor|ActorHasTag OtherActor "Small")
    (Actor|DestroyActor OtherActor)
    (Development|PrintString "Hit Small Target")
    (Audio|PlaySound2D "/Game/StarterContent/Audio/Collapse01.Collapse01" 1.0 1.0 0.0 0 0)
    (Actor|DestroyActor)
    (Variables|/Game/Dynamic/Stages/Fun/Blueprints/BP_FunCharacter.BP_FunCharacter_C|SetScoreToAdd _as_bp_fun_character 25.0)
    (Default|UpdateScore _as_bp_fun_character)
    (bind _result (Math|Integer|DecrementInt (Variables|/Game/Dynamic/Stages/Fun/Blueprints/BP_FunCharacter.BP_FunCharacter_C|GetTargetsRemaining _as_bp_fun_character))
      (:%20%20
        (Variables|/Game/Dynamic/Stages/Fun/Blueprints/BP_FunCharacter.BP_FunCharacter_C|SetTargetsRemaining _as_bp_fun_character _result)))
    (elif (Actor|ActorHasTag OtherActor "Med")
      (Actor|DestroyActor OtherActor)
      (Development|PrintString "Hit Med Target")
      (Audio|PlaySound2D "/Game/StarterContent/Audio/Collapse01.Collapse01" 1.0 1.0 0.0 0 0)
      (Actor|DestroyActor)
      (Variables|/Game/Dynamic/Stages/Fun/Blueprints/BP_FunCharacter.BP_FunCharacter_C|SetScoreToAdd _as_bp_fun_character_3 5e+01)
      (Default|UpdateScore _as_bp_fun_character_3)
      (bind _result_2 (Math|Integer|DecrementInt (Variables|/Game/Dynamic/Stages/Fun/Blueprints/BP_FunCharacter.BP_FunCharacter_C|GetTargetsRemaining _as_bp_fun_character_3))
        (:%20%20
          (Variables|/Game/Dynamic/Stages/Fun/Blueprints/BP_FunCharacter.BP_FunCharacter_C|SetTargetsRemaining _as_bp_fun_character_3 _result_2)))
      (elif (Actor|ActorHasTag OtherActor "Large")
        (Actor|DestroyActor OtherActor)
        (Development|PrintString "Hit Large Target")
        (Audio|PlaySound2D "/Game/StarterContent/Audio/Collapse01.Collapse01" 1.0 1.0 0.0 0 0)
        (Actor|DestroyActor)
        (Variables|/Game/Dynamic/Stages/Fun/Blueprints/BP_FunCharacter.BP_FunCharacter_C|SetScoreToAdd _as_bp_fun_character_2 2e+02)
        (Default|UpdateScore _as_bp_fun_character_2)
        (bind _result_3 (Math|Integer|DecrementInt (Variables|/Game/Dynamic/Stages/Fun/Blueprints/BP_FunCharacter.BP_FunCharacter_C|GetTargetsRemaining _as_bp_fun_character_2))
          (:%20%20
            (Variables|/Game/Dynamic/Stages/Fun/Blueprints/BP_FunCharacter.BP_FunCharacter_C|SetTargetsRemaining _as_bp_fun_character_2 _result_3)))
        (else
          (Development|PrintString "Nothing Hit")
          (Actor|DestroyActor))))))

(event EventBeginPlay
  (Utilities|FlowControl|DoOnce false
    (:Completed
      (bind _asbp_fun_character (Utilities|Casting|CastToBP_FunCharacter (Game|GetPlayerCharacter 0)))
      (Variables|Default|SetAs%20BP%20Fun%20Character _asbp_fun_character))))

(event Collision|EventActorBeginOverlap
  (params (OtherActor :type Actor%20Object%20Reference)))

(event EventTick
  (params (DeltaSeconds :type Float%20%28single-precision%29)))

(fn ConstructionScript)