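; BP_FileTarget is a file target in the Fun stage that may slide sideways and is removed when something overlaps its box.
; After a short delay, a random roll decides whether it moves, using BP_MoveBounds for its Y limits.
; The Movement timeline ping-pongs through a FlipFlop, starting from the spawn position on the first pass.
; The first overlap stops movement, and the Kill timeline sinks the target before destroying it.
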(event OnComponentBeginOverlap(Box)
  (params (OverlappedComponent :type Primitive%20Component%20Object%20Reference) (OtherActor :type Actor%20Object%20Reference) (OtherComp :type Primitive%20Component%20Object%20Reference) (OtherBodyIndex :type Integer) (bFromSweep :type Boolean) (SweepResult :type Hit%20Result%20Structure%20%28by%20ref%29))
  (Utilities|FlowControl|DoOnce false
    (:Completed
      (CallFunction|KillFile))))

(event Custom|StartMoving
  (bind _moveboundsref (Variables|Default|GetMoveBoundsRef))
  (bind _scene (Variables|Default|GetScene))
  (bind _scene_2 (Variables|Default|GetScene))
  (bind _returnvalue (Transformation|GetWorldLocation _scene_2))
  (bind _returnvalue_2 (Transformation|GetWorldLocation _scene))
  (bind _movement (Timeline|Movement PlayFromStart)
    (:Update
      (if (Variables|Default|GetJustSpawned)
        (Transformation|SetWorldLocation _scene (Math|Vector|MakeVector (.x _returnvalue_2) (Math|Float|Lerp (Variables|Default|GetStart%20Y%20Location) (Variables|/Game/Dynamic/Stages/Fun/Blueprints/BP_MoveBounds.BP_MoveBounds_C|GetRightBoundsY (Variables|Default|GetMoveBoundsRef)) _movement) (.z _returnvalue_2)) false false)
        (else
          (Transformation|SetWorldLocation _scene_2 (Math|Vector|MakeVector (.x _returnvalue) (Math|Float|Lerp (Variables|/Game/Dynamic/Stages/Fun/Blueprints/BP_MoveBounds.BP_MoveBounds_C|GetLeftBoundsY _moveboundsref) (Variables|/Game/Dynamic/Stages/Fun/Blueprints/BP_MoveBounds.BP_MoveBounds_C|GetRightBoundsY _moveboundsref) _movement) (.z _returnvalue)) false false))))
    (:Finished
      (Utilities|FlowControl|FlipFlop
        (:A
          (Variables|Default|SetJustSpawned false)
          (CallFunction|ReverseMovement))
        (:B
          (CallFunction|StartMoving))))))

(event Custom|ReverseMovement
  (bind _moveboundsref (Variables|Default|GetMoveBoundsRef))
  (bind _scene (Variables|Default|GetScene))
  (bind _scene_2 (Variables|Default|GetScene))
  (bind _returnvalue (Transformation|GetWorldLocation _scene_2))
  (bind _returnvalue_2 (Transformation|GetWorldLocation _scene))
  (bind _movement (Timeline|Movement ReverseFromEnd)
    (:Update
      (if (Variables|Default|GetJustSpawned)
        (Transformation|SetWorldLocation _scene (Math|Vector|MakeVector (.x _returnvalue_2) (Math|Float|Lerp (Variables|Default|GetStart%20Y%20Location) (Variables|/Game/Dynamic/Stages/Fun/Blueprints/BP_MoveBounds.BP_MoveBounds_C|GetRightBoundsY (Variables|Default|GetMoveBoundsRef)) _movement) (.z _returnvalue_2)) false false)
        (else
          (Transformation|SetWorldLocation _scene_2 (Math|Vector|MakeVector (.x _returnvalue) (Math|Float|Lerp (Variables|/Game/Dynamic/Stages/Fun/Blueprints/BP_MoveBounds.BP_MoveBounds_C|GetLeftBoundsY _moveboundsref) (Variables|/Game/Dynamic/Stages/Fun/Blueprints/BP_MoveBounds.BP_MoveBounds_C|GetRightBoundsY _moveboundsref) _movement) (.z _returnvalue)) false false))))
    (:Finished
      (Utilities|FlowControl|FlipFlop
        (:A
          (Variables|Default|SetJustSpawned false)
          (CallFunction|ReverseMovement))
        (:B
          (CallFunction|StartMoving))))))

(event Custom|KillFile
  (bind _scene (Variables|Default|GetScene))
  (bind _returnvalue (Transformation|GetWorldLocation _scene))
  (Audio|Components|Audio|Stop (Variables|Default|GetMovement))
  (bind _newtrack_0 (Timeline|Kill PlayFromStart)
    (:Update
      (Transformation|SetWorldLocation _scene (Math|Vector|MakeVector (.x _returnvalue) (.y _returnvalue) (Math|Float|Lerp (.z _returnvalue) (- (.z _returnvalue) 1.5e+02) _newtrack_0)) false false))
    (:Finished
      (Actor|DestroyActor))))

(event EventBeginPlay
  (|CallParentFunction)
  (Utilities|FlowControl|Delay 1.0)
  (switch int (Math|Random|RandomIntegerinRange 0 1)
    (:0
      (bind _returnvalue (Actor|GetActorOfClass "/Game/Dynamic/Stages/Fun/Blueprints/BP_MoveBounds.BP_MoveBounds_C"))
      (Variables|Default|SetMoveBoundsRef _returnvalue)
      (Variables|Default|SetStart%20Y%20Location (.y (Transformation|GetWorldLocation (Variables|Default|GetScene))))
      (CallFunction|StartMoving))))

(event Collision|EventActorBeginOverlap
  (params (OtherActor :type Actor%20Object%20Reference))
  (|CallParentFunction OtherActor) ; This node is disabled and will not be called.\nDrag off pins to build functionality.
)

(event EventTick
  (params (DeltaSeconds :type Float%20%28single-precision%29))
  (|CallParentFunction DeltaSeconds) ; This node is disabled and will not be called.\nDrag off pins to build functionality.
)

(fn ConstructionScript
  (|CallParentFunction))